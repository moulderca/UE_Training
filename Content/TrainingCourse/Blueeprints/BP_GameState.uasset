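; BP_GameState tracks shape interactions in a training course and toggles a HUD notification when three reported IDs match.
; On BeginPlay it caches the BP_HUD actor and binds to the state-updated dispatcher of every StaticMeshActor's AC_Interaction component.
; OnShapesUpdated collects incoming IDs; on the third, CompareResults checks they are identical, then clears the list whatever the outcome.
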(event `self.ReceiveBeginPlay`
  (`self.Setup`))

(event `OnShapesUpdated`
  (params (ID :type Integer))
  (bind _returnvalue (`KismetArrayLibrary.Array_Add` (`self.Results`) ID))
  (if (== _returnvalue 2)
    (`self.CompareResults`)))

(fn `CompareResults`
  (bind _results (`self.Results`))
  (bind _output (`|GetArrayItem` _results))
  (if (and (== _output (`|GetArrayItem` _results 1)) (== _output (`|GetArrayItem` _results 2)))
    (`/Game/TrainingCourse/Blueeprints/BP_HUD.ToggleNotification` (`self.HUD`)))
  (`KismetArrayLibrary.Array_Clear` (`self.Results`)))

(fn `Setup`
  (`|ExecutionSequence`
    (:`then_0`
      (bind _outactors (`GameplayStatics.GetAllActorsOfClass` "/Script/Engine.StaticMeshActor"))
      (for _array_element _outactors
        (bind _returnvalue (`self.GetComponentByClass` _array_element "/Game/TrainingCourse/Blueeprints/AC_Interaction.AC_Interaction_C"))
        (`/Engine/EditorBlueprintResources/StandardMacros.IsValid` _returnvalue
          (:`Is Valid`
            (add `/Game/TrainingCourse/Blueeprints/AC_Interaction.ED_StateUpdated` _returnvalue (`|CreateDelegate` :!event `OnShapesUpdated`))))))
    (:`then_1`
      (bind _returnvalue_2 (`GameplayStatics.GetActorOfClass` "/Game/TrainingCourse/Blueeprints/BP_HUD.BP_HUD_C"))
      (set `self.HUD` _returnvalue_2))))

(fn `UserConstructionScript`)