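; Actor component for a Static Mesh Actor that changes the owner's shape in response to triggers.
; On BeginPlay it caches the owner and binds a shape-change event on every BP_TriggerBase in the level.
; The change handler picks a random NewMesh entry, applies it and broadcasts the index through the state-updated dispatcher.
; An invalid index prints debug messages and resets to the first mesh.
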(event `self.ReceiveBeginPlay`
  (bind _asstatic_mesh_actor (cast `StaticMeshActor` (`self.GetOwner`)))
  (set `self.StaticMeshActor` _asstatic_mesh_actor)
  (bind _outactors (`GameplayStatics.GetAllActorsOfClass` "/Game/TrainingCourse/Blueeprints/BP_TriggerBase.BP_TriggerBase_C"))
  (for _array_element _outactors
    (add `/Game/TrainingCourse/Blueeprints/BP_TriggerBase.ChangeShape` _array_element (`|CreateDelegate` :!event `OnChangeSape`))))

(event `OnChangeSape`
  (bind _currentid (`self.CurrentID`))
  (set `self.CurrentID` (`KismetMathLibrary.RandomIntegerInRange` 0 (`KismetArrayLibrary.Array_LastIndex` (`self.New Mesh`))))
  (`self.ChangeStatcMeshActor` (`self.StaticMeshActor`) _currentid)
  (`self.ED_StateUpdated` _currentid))

(fn `ChangeStatcMeshActor`
  (params (StaticMeshActor :type "StaticMeshActor Object Reference") (Index :type Integer))
  (bind _new_mesh (`self.New Mesh`))
  (bind _debug (`self.Debug`))
  (if (`KismetArrayLibrary.Array_IsValidIndex` _new_mesh Index)
    (`StaticMeshComponent.SetStaticMesh` (`StaticMeshActor.StaticMeshComponent` StaticMeshActor) (`|GetArrayItem` _new_mesh Index))
    (else
      (`KismetSystemLibrary.PrintString` (`KismetStringLibrary.Concat_StrStr` "WrongIndex" (`KismetStringLibrary.Conv_IntToString` Index)) _debug)
      (`self.Reset`)
      (`KismetSystemLibrary.PrintString` "StateReset" _debug))))

(fn `Reset`
  (`self.ChangeStatcMeshActor` (`self.StaticMeshActor`)))